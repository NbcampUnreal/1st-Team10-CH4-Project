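; Anim notify state that runs melee-style hit detection on each tick of its window by calling ServerPerformHitCheck on the owner's CSCombatComponent.
; For AI characters it fires only while a hit is pending, using the trace points, damage and type stored on the component.
; For other CSBaseCharacter owners it fires only when locally controlled, combining the notify's own trace names and launch type with the component's current attack damage.
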(fn `Received_NotifyTick`
  (params (MeshComp :type "SkeletalMeshComponent Object Reference") (Animation :type "AnimSequenceBase Object Reference") (FrameDeltaTime :type "Float (single-precision)") (EventReference :type "AnimNotifyEventReference Structure (by ref)"))
  (returns (ReturnValue :type Boolean))
  (locals (CombatComponent :type "CSCombatComponent Object Reference"))
  (bind _returnvalue (`ActorComponent.GetOwner` MeshComp))
  (bind _returnvalue_2 (`Actor.GetComponentByClass` _returnvalue "/Script/CS.CSCombatComponent"))
  (bind _asaibase_character (cast `AIBaseCharacter` _returnvalue)
    (:`then`
      (bind _returnvalue_3 (`Actor.GetComponentByClass` _asaibase_character "/Script/CS.CSCombatComponent"))
      (if (`CSCombatComponent.IsPendingHit` _returnvalue_3)
        (`CSCombatComponent.Server_PerformHitCheck` _returnvalue_3 (`CSCombatComponent.GetPendingTraceStart` _returnvalue_3) (`CSCombatComponent.GetPendingTraceEnd` _returnvalue_3) (`CSCombatComponent.GetPendingDamage` _returnvalue_3) (`CSCombatComponent.GetPendingDType` _returnvalue_3))
        (return false)))
    (:`CastFailed`
      (bind _ascsbase_character (cast `CSBaseCharacter` _returnvalue))
      (`/Engine/EditorBlueprintResources/StandardMacros.IsValid` _ascsbase_character
        (:`Is Valid`
          (if (`Pawn.IsLocallyControlled` _ascsbase_character)
            (`/Engine/EditorBlueprintResources/StandardMacros.IsValid` _returnvalue_2
              (:`Is Valid`
                (`CSCombatComponent.Server_PerformHitCheck` _returnvalue_2 (`self.Trace Start Name`) (`self.Trace End Name`) (`CSCombatComponent.GetCurrentAttackDamage` _returnvalue_2) (cast `ELaunchTypes` (`self.DType`)))
                (return false)))))))))